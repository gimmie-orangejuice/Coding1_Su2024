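; BP_CanOfBeans is a pickup item that the custom third-person character can hold, drop and use.
; Overlapping its trigger asks the character to pick it up; Pickup then attaches the root to the ik_hand_r socket.
; Drop detaches it and enables physics on the can, but sets collision to NoCollision.
; PrimaryAction only prints a health-gain message; the logic to clear HeldItem and destroy the actor is disconnected.
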(event OnComponentBeginOverlap(PickUpTriger)
  (params (OverlappedComponent :type Primitive%20Component%20Object%20Reference) (OtherActor :type Actor%20Object%20Reference) (OtherComp :type Primitive%20Component%20Object%20Reference) (OtherBodyIndex :type Integer) (bFromSweep :type Boolean) (SweepResult :type Hit%20Result%20Structure%20%28by%20ref%29))
  (bind _asbp_third_person_character_custom (Utilities|Casting|CastToBP_ThirdPersonCharacterCUSTOM OtherActor))
  (Default|TrytoPickUp _asbp_third_person_character_custom self))

(event EventBeginPlay)

(event Collision|EventActorBeginOverlap
  (params (OtherActor :type Actor%20Object%20Reference)))

(event EventTick
  (params (DeltaSeconds :type Float%20%28single-precision%29)))

(event EventPickup
  (params (ParentMesh :type Skeletal%20Mesh%20Component%20Object%20Reference))
  (Transformation|AttachComponentToComponent (Variables|Default|GetDefaultSceneRoot) ParentMesh "ik_hand_r" "SnapToTarget" "KeepRelative" "KeepRelative" true))

(event EventDrop
  (Transformation|DetachFromComponent (Variables|Default|GetDefaultSceneRoot) "KeepRelative" "KeepRelative" "KeepRelative" true)
  (Physics|SetSimulatePhysics (Variables|Default|GetCan) true)
  (Collision|SetCollisionEnabled (Variables|Default|GetCan) "NoCollision"))

(event EventPrimaryAction
  (params (RefTirdCharCUSTOM :type BP%20Third%20Person%20Character%20CUSTOM%20Object%20Reference))
  (Development|PrintString "You've gained 10 health"))

(fn ConstructionScript)