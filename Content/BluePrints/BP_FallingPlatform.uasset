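; BP_FallingPlatform is a platform that falls after activation, then returns to its starting transform.
; Activate, when Ready, waits briefly before Drop enables physics on the Cube, and Reset follows after another delay.
; Reset disables physics and uses a Timeline to lerp the Cube back, swapping state materials and restoring Ready when finished.
; The Box overlap only casts to the player character; nothing here calls Activate.
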(event OnComponentBeginOverlap(Box)
  (params (OverlappedComponent :type Primitive%20Component%20Object%20Reference) (OtherActor :type Actor%20Object%20Reference) (OtherComp :type Primitive%20Component%20Object%20Reference) (OtherBodyIndex :type Integer) (bFromSweep :type Boolean) (SweepResult :type Hit%20Result%20Structure%20%28by%20ref%29))
  (Utilities|Casting|CastToBP_ThirdPersonCharacterCUSTOM OtherActor))

(event Custom|Activate
  ;[0.7993 1 0.7463] Player activated the platform by standing on it
  (if (Variables|Default|GetReady)
    (Development|PrintString "1 secound left")
    (Variables|Default|SetReady false)
    (Utilities|FlowControl|Delay 1.0)
    (CallFunction|Drop)))

(event Custom|Drop
  ;[1 0.5045 0.6939] platform drops
  (Development|PrintString "Dropping")
  (Physics|SetSimulatePhysics (Variables|Default|GetCube) true)
  (Rendering|Material|SetMaterial (Variables|Default|GetCube) 0 "/Game/Materials/MI_PlayformFAlling.MI_PlayformFAlling")
  (Utilities|FlowControl|Delay 3.0)
  (Class|TypedElementListLibrary|Reset))

(event Custom|Reset
  ;[1 1 1] Platform goes back to starting position
  (Development|PrintString "reseting")
  (Variables|Default|Set%20Reset%20transform (Transformation|GetWorldTransform (Variables|Default|GetCube)))
  (Physics|SetSimulatePhysics (Variables|Default|GetCube) false)
  (Rendering|Material|SetMaterial (Variables|Default|GetCube) 0 "/Game/Materials/MI_PlayformResting.MI_PlayformResting")
  (bind _newtrack_0 (Timeline|Timeline Play)
    (:Update
      (Transformation|SetWorldLocationAndRotation (Variables|Default|GetCube) (.location (Math|Transform|Lerp(Transform) (Variables|Default|Get%20Reset%20transform) (Variables|Default|GetStartingTransform) _newtrack_0)) (.rotation (Math|Transform|Lerp(Transform) (Variables|Default|Get%20Reset%20transform) (Variables|Default|GetStartingTransform) _newtrack_0)) false false)
      (Rendering|Material|SetMaterial (Variables|Default|GetCube) 0 "/Game/Materials/MI_PlatformReady.MI_PlatformReady"))
    (:Finished
      (Variables|Default|SetReady true))))

(event EventBeginPlay
  (Variables|Default|SetStartingTransform (Transformation|GetWorldTransform (Variables|Default|GetCube))) ; saveing the starting rotation and location of cube
)

(event Collision|EventActorBeginOverlap
  (params (OtherActor :type Actor%20Object%20Reference)))

(event EventTick
  (params (DeltaSeconds :type Float%20%28single-precision%29)))

(fn ConstructionScript)