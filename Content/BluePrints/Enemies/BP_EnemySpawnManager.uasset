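; BP_EnemySpawnManager runs endless enemy waves from the spawner actors placed in the level.
; On BeginPlay it gathers all BP_EnemySpawner actors, then spawns one BP_Enemy at each, passing itself as the enemy's manager and counting the total.
; RemovEnemyeandCheck decrements that count and, when none remain, announces a new wave on screen and respawns all enemies after a short delay.
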(event Custom|Spawn%20Enemies
  (for _array_element (Variables|Default|GetSpawnsers)
    (bind _returnvalue (Game|SpawnActorfromClass "/Game/BluePrints/Enemies/BP_Enemy.BP_Enemy_C" (Math|Transform|MakeTransform (.location (Transformation|GetWorldTransform (Variables|/Game/BluePrints/Enemies/BP_EnemySpawner.BP_EnemySpawner_C|GetDefaultSceneRoot _array_element))) (.rotation (Transformation|GetWorldTransform (Variables|/Game/BluePrints/Enemies/BP_EnemySpawner.BP_EnemySpawner_C|GetDefaultSceneRoot _array_element))) "1.000000,1.000000,1.000000") "Undefined" "MultiplyWithRoot" 0 0)) ; create new enemy at spawner location and roation
    (Variables|/Game/BluePrints/Enemies/BP_Enemy.BP_Enemy_C|SetEnemyManager _returnvalue self) ; Assign the manager variable to each enemy
    (Math|Integer|IncrementInt (Variables|Default|GetCurrentEnemy%20Total))))

(event Custom|RemovEnemyeandCheck
  (Math|Integer|DecrementInt (Variables|Default|GetCurrentEnemy%20Total)
    (:%20%20
      (if (not (> (Variables|Default|GetCurrentEnemy%20Total) 0))
        (Development|PrintString "New wave incomeing" true true "(R=1.000000,G=0.105386,B=0.000000,A=1.000000)" 5.0)
        (Utilities|FlowControl|Delay 5.0)
        (CallFunction|SpawnEnemies)))))

(event EventBeginPlay
  (Utilities|FlowControl|Sequence
    (:then_0
      (Development|PrintString "Enemy Spawn Manager is Ready")
      (bind _outactors (Actor|GetAllActorsOfClass "/Game/BluePrints/Enemies/BP_EnemySpawner.BP_EnemySpawner_C"))
      (Variables|Default|SetSpawnsers _outactors))
    (:then_1
      (CallFunction|SpawnEnemies))))

(event Collision|EventActorBeginOverlap
  (params (OtherActor :type Actor%20Object%20Reference)))

(event EventTick
  (params (DeltaSeconds :type Float%20%28single-precision%29)))

(fn ConstructionScript)