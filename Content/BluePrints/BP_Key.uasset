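; BP_Key is a collectible key pickup for the custom third-person character.
; When its box collision overlaps a BP_ThirdPersonCharacterCUSTOM, it increments that character's KeyCount and destroys itself.
; Debug strings report spawning, the pickup, the new key total and failed casts.
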(event OnComponentBeginOverlap(BoxColision)
  (params (OverlappedComponent :type Primitive%20Component%20Object%20Reference) (OtherActor :type Actor%20Object%20Reference) (OtherComp :type Primitive%20Component%20Object%20Reference) (OtherBodyIndex :type Integer) (bFromSweep :type Boolean) (SweepResult :type Hit%20Result%20Structure%20%28by%20ref%29))
  (bind _asbp_third_person_character_custom (Utilities|Casting|CastToBP_ThirdPersonCharacterCUSTOM OtherActor)
    (:then
      (Development|PrintString "player ran though key" true true "(R=0.000000,G=0.660000,B=1.000000,A=1.000000)" 5.0)
      (Variables|/Game/BluePrints/BP_ThirdPersonCharacterCUSTOM.BP_ThirdPersonCharacterCUSTOM_C|SetkeyCount _asbp_third_person_character_custom (+ (Variables|/Game/BluePrints/BP_ThirdPersonCharacterCUSTOM.BP_ThirdPersonCharacterCUSTOM_C|GetkeyCount _asbp_third_person_character_custom) 1)) ; set key count to 1
      (Development|PrintString (Utilities|String|Append "The Player has " (Utilities|String|ToString(Integer) (Variables|/Game/BluePrints/BP_ThirdPersonCharacterCUSTOM.BP_ThirdPersonCharacterCUSTOM_C|GetkeyCount _asbp_third_person_character_custom)) " keys"))
      (Actor|DestroyActor) ; destory key
    )
    (:CastFailed
      (Development|PrintString "cast failed" true true "(R=1.000000,G=0.000000,B=0.005851,A=1.000000)" 5.0))))

(event EventBeginPlay
  (Development|PrintString "this key exists"))

(event Collision|EventActorBeginOverlap
  (params (OtherActor :type Actor%20Object%20Reference)))

(event EventTick
  (params (DeltaSeconds :type Float%20%28single-precision%29)))

(fn ConstructionScript)