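; BP_MoveingPlatform is a platform actor that moves back and forth endlessly between its Start and End components.
; After a short delay on BeginPlay, a Timeline drives a lerp of the Platform's relative location between those two points, without sweeping.
; Each time the Timeline finishes, it pauses, then a FlipFlop alternates between reversing and replaying it, printing the travel direction.
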(event EventBeginPlay
  (Utilities|FlowControl|Delay 2.0)
  (bind _newtrack_0 (Timeline|Timeline PlayFromStart)
    (:Update
      (Transformation|SetRelativeLocation (Variables|Default|GetPlatform) (Math|Vector|Lerp(Vector) (Variables|/Script/Engine.SceneComponent|GetRelativeLocation (Variables|Default|GetStart)) (Variables|/Script/Engine.SceneComponent|GetRelativeLocation (Variables|Default|GetEnd)) _newtrack_0) false false))
    (:Finished
      (Utilities|FlowControl|Delay 2.0)
      (Utilities|FlowControl|FlipFlop
        (:A
          (Development|PrintString "going to the start")
          (Timeline|Timeline ReverseFromEnd))
        (:B
          (Development|PrintString "going to the end")
          (Timeline|Timeline PlayFromStart))))))

(event Collision|EventActorBeginOverlap
  (params (OtherActor :type Actor%20Object%20Reference)))

(event EventTick
  (params (DeltaSeconds :type Float%20%28single-precision%29)))

(fn ConstructionScript)